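; BP_AshCharacter is a character Blueprint that changes outfit overlay materials in response to speed and damage boost events.
; BeginPlay caches the first material of the shoes, lower and upper outfit meshes.
; Speed boost start applies a green overlay to lower and shoes, and its end sets their cached materials as overlays.
; Both damage boost events set the cached materials as overlays on all three meshes, so neither applies a distinct color.
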(event `self.ReceiveBeginPlay`
  (set `self.ShoeFirst` (`PrimitiveComponent.GetMaterial` (`self.OutfitShoes`) 0))
  (set `self.LowerFirst` (`PrimitiveComponent.GetMaterial` (`self.OutfitLower`) 0))
  (set `self.UpperFirst` (`PrimitiveComponent.GetMaterial` (`self.OutfitUpper`) 0)))

(event `self.OnSpeedBoostStarted`
  (params (SpeedMultiplier :type "Float (single-precision)") (JumpMultiplier :type "Float (single-precision)") (Duration :type "Float (single-precision)"))
  (`MeshComponent.SetOverlayMaterial` (`self.OutfitLower`) "/Game/CoreC/03Outfit/000_TechwearRunnerCourier01/Materials/Green.Green")
  (`MeshComponent.SetOverlayMaterial` (`self.OutfitShoes`) "/Game/CoreC/03Outfit/000_TechwearRunnerCourier01/Materials/Green.Green"))

(event `self.OnSpeedBoostEnded`
  (`MeshComponent.SetOverlayMaterial` (`self.OutfitLower`) (`self.LowerFirst`))
  (`MeshComponent.SetOverlayMaterial` (`self.OutfitShoes`) (`self.ShoeFirst`)))

(event `self.OnDamageBoostStarted`
  (params (DamageMultiplierValue :type "Float (single-precision)") (Duration :type "Float (single-precision)"))
  (`MeshComponent.SetOverlayMaterial` (`self.OutfitShoes`) (`self.ShoeFirst`))
  (`MeshComponent.SetOverlayMaterial` (`self.OutfitUpper`) (`self.UpperFirst`))
  (`MeshComponent.SetOverlayMaterial` (`self.OutfitLower`) (`self.LowerFirst`)))

(event `self.OnDamageBoostEnded`
  (`MeshComponent.SetOverlayMaterial` (`self.OutfitShoes`) (`self.ShoeFirst`))
  (`MeshComponent.SetOverlayMaterial` (`self.OutfitUpper`) (`self.UpperFirst`))
  (`MeshComponent.SetOverlayMaterial` (`self.OutfitLower`) (`self.LowerFirst`)))

(fn `UserConstructionScript`)